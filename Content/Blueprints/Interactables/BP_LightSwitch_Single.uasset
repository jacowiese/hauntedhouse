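; BP_LightSwitch_Single is an interactable single light switch that toggles its LightState flag on each Interact event.
; ReflectState poses the Switch component to match that flag with a slight rotation and offset, snapping instantly without animation.
; The Construction Script runs the same function, so the placed switch shows its initial state.
; The graphs change only the switch's pose and drive no light.
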(event EventInteract
  (params (PlayerCharacter :type First%20Person%20Character%20Object%20Reference))
  (if (Variables|Default|GetLightState)
    (Variables|Default|SetLightState false)
    (else
      (Variables|Default|SetLightState true)))
  (CallFunction|ReflectState))

(fn ConstructionScript
  (CallFunction|ReflectState))

(fn ReflectState
  (bind _switch (Variables|Default|GetSwitch))
  (if (Variables|Default|GetLightState)
    (Transformation|SetRelativeRotation _switch "-3.000000, 0, 0" false false)
    (Transformation|SetRelativeLocation _switch "-0.015000,0.000000, 0" false false)
    (else
      (Transformation|SetRelativeRotation _switch "0, 0, 0" false false)
      (Transformation|SetRelativeLocation _switch "0, 0, 0" false false))))